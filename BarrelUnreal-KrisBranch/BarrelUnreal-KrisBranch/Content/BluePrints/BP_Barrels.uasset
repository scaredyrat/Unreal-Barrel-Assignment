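; Barrel actor that takes a random flesh, plastic or wooden look and explodes when the game mode signals destruction.
; The construction script creates a dynamic instance of MI_Barrel and randomly swaps its ARM, base color and normal textures, so one Blueprint covers all three variants.
; On BeginPlay it binds to the destroy dispatcher in GM_Barrels, whose call spawns an explosion emitter at the barrel and destroys the actor.
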(event Custom|CE_Destroy
  (Effects|SpawnEmitteratLocation "/Game/FX/Particles/PS_ImpactExplosion3.PS_ImpactExplosion3" (Transformation|GetActorLocation))
  (Actor|DestroyActor))

(event EventBeginPlay
  (bind _asgm_barrels (Utilities|Casting|CastToGM_Barrels (Game|GetGameMode)))
  (Variables|Default|SetGameModeRef _asgm_barrels)
  (EventDispatchers|BindEventtoEDDestroy (Variables|Default|GetGameModeRef) (delegate Custom|CE_Destroy)))

(fn ConstructionScript
  (bind _returnvalue (Rendering|Material|CreateDynamicMaterialInstance (Variables|Default|GetBarrel) 0 "/Game/TexMatt/MI_Barrel.MI_Barrel" "None" :!class /Script/Engine.PrimitiveComponent))
  (Variables|Default|SetDyna%20Material _returnvalue)
  (switch int (Math|Random|RandomIntegerinRange 0 2)
    (:0
      (Rendering|Material|SetTextureParameterValue (Variables|Default|GetDyna%20Material) "ARM" "/Game/TexMatt/FleshBarrel_ARM.FleshBarrel_ARM")
      (Rendering|Material|SetTextureParameterValue (Variables|Default|GetDyna%20Material) "BaseColor" "/Game/TexMatt/FleshBarrel_Color.FleshBarrel_Color")
      (Rendering|Material|SetTextureParameterValue (Variables|Default|GetDyna%20Material) "Normal" "/Game/TexMatt/FleshBarrel_Normal.FleshBarrel_Normal"))
    (:1
      (Rendering|Material|SetTextureParameterValue (Variables|Default|GetDyna%20Material) "ARM" "/Game/TexMatt/PlasticBarrel_ARM.PlasticBarrel_ARM")
      (Rendering|Material|SetTextureParameterValue (Variables|Default|GetDyna%20Material) "BaseColor" "/Game/TexMatt/PlasticBarrel_Color.PlasticBarrel_Color")
      (Rendering|Material|SetTextureParameterValue (Variables|Default|GetDyna%20Material) "Normal" "/Game/TexMatt/PlasticBarrel_Normal.PlasticBarrel_Normal"))
    (:2
      (Rendering|Material|SetTextureParameterValue (Variables|Default|GetDyna%20Material) "ARM" "/Game/TexMatt/WoodenBarrel_ARM.WoodenBarrel_ARM")
      (Rendering|Material|SetTextureParameterValue (Variables|Default|GetDyna%20Material) "BaseColor" "/Game/TexMatt/WoodenBarrel_Color.WoodenBarrel_Color")
      (Rendering|Material|SetTextureParameterValue (Variables|Default|GetDyna%20Material) "Normal" "/Game/TexMatt/WoodenBarrel_Normal.WoodenBarrel_Normal"))))